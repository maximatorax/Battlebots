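; BP_BotPlayer is a player pawn with Enhanced Input movement and a test attack through the Gameplay Ability System.
; BeginPlay adds the player mapping context to its player controller's input subsystem.
; Move inputs apply movement along control-rotation right and forward vectors, with pitch zeroed.
; Attack tries to activate GA_AttackTest, then immediately calls EndAbility on every ability in the Ability System Component.
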(event Input|EnhancedActionEvents|EnhancedInputActionIA_MoveForwardBackward
  (params (ActionValue :type Float%20%28double-precision%29) (ElapsedSeconds :type Float%20%28double-precision%29) (TriggeredSeconds :type Float%20%28double-precision%29) (InputAction :type Input%20Action%20Object%20Reference :default "/Game/Inputs/IA_MoveForwardBackward.IA_MoveForwardBackward"))
  ;[1 1 1] Move Forward/Backward
  (Pawn|Input|AddMovementInput (Math|Vector|GetForwardVector (Math|Rotator|MakeRotator 0.0 0.0 (.yaw (Pawn|GetControlRotation :!class /Script/Engine.Pawn)))) ActionValue false))

(event Input|EnhancedActionEvents|EnhancedInputActionIA_MoveLeftRight
  (params (ActionValue :type Float%20%28double-precision%29) (ElapsedSeconds :type Float%20%28double-precision%29) (TriggeredSeconds :type Float%20%28double-precision%29) (InputAction :type Input%20Action%20Object%20Reference :default "/Game/Inputs/IA_MoveLeftRight.IA_MoveLeftRight"))
  (bind _returnvalue (Pawn|GetControlRotation :!class /Script/Engine.Pawn))
  ;[1 1 1] Move Left/Right
  (Pawn|Input|AddMovementInput (Math|Vector|GetRightVector (Math|Rotator|MakeRotator (.roll _returnvalue) 0.0 (.yaw _returnvalue))) ActionValue false))

(event Input|EnhancedActionEvents|EnhancedInputActionIA_Attack
  (params (ActionValue :type Boolean) (ElapsedSeconds :type Float%20%28double-precision%29) (TriggeredSeconds :type Float%20%28double-precision%29) (InputAction :type Input%20Action%20Object%20Reference :default "/Game/Inputs/IA_Attack.IA_Attack"))
  (bind _returnvalue (Ability|GetAbilitySystemComponent 0))
  (:Started
    (Abilities|TryActivateAbilitybyClass _returnvalue "/Game/Abilities/GA_AttackTest.GA_AttackTest_C" true)
    (bind _outabilityhandles (Class|AbilitySystemComponent|GetAllAbilities _returnvalue))
    (for _array_element _outabilityhandles
      (Ability|EndAbility (.ReturnValue (Ability|GameplayAbility|GetGameplayAbilityfromSpecHandle _returnvalue _array_element))))))

(event EventBeginPlay
  ;[1 1 1] Setup Enhanced Input System
  (bind _asplayer_controller (Utilities|Casting|CastToPlayerController (Pawn|GetController)))
  (bind _output_get (Variables|Default|SetPlayerController _asplayer_controller))
  (Input|AddMappingContext (PlayerController|LocalPlayerSubsystems|GetEnhancedInputLocalPlayerSubsystem _output_get) "/Game/Inputs/IMC_PlayerMappingContext.IMC_PlayerMappingContext" 0 "(bIgnoreAllPressedKeysUntilRelease=True,bForceImmediately=False,bNotifyUserSettings=False)"))

(fn ConstructionScript)