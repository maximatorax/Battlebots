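; Game instance for Battlebots that handles hosting, joining and starting multiplayer sessions through BBSessionSubsystem.
; Hosting creates a session with two public connections and opens the Lobby level as a listen server.
; Joining searches for a single session and joins it, while starting the game calls StartSession on the subsystem.
; Session failures and successful joins are reported only through PrintString.
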(event Custom|Instance_HostSession
  (params (Host :type Player%20Controller%20Object%20Reference))
  ;[1 1 1] Host Session
  (|Session (Subsystems|GetBBSessionSubsystem) Host 2 false
    (:OnSuccess
      (Game|OpenLevel(byName) "Lobby" true "listen"))
    (:OnFailure
      (Development|PrintString "Could Not Create Session"))))

(event Custom|Instance_FindAndJoinSession
  (params (Host :type Player%20Controller%20Object%20Reference))
  (bind _returnvalue (Subsystems|GetBBSessionSubsystem))
  ;[1 1 1] Find/Join Session
  (bind _results (|FindSessions _returnvalue Host 1 false)
    (:OnSuccess
      (for _array_element _results
        (Variables|Default|SetSessions _array_element))
      (|JoinSession _returnvalue Host (Variables|Default|GetSessions)
        (:OnSuccess
          (Development|PrintString "Session Joined"))
        (:OnFailure
          (Development|PrintString "Unable To Join"))))
    (:OnFailure
      (Development|PrintString "Session Not Found"))))

(event Custom|Instance_StartGame
  (Class|BBSessionSubsystem|StartSession (Subsystems|GetBBSessionSubsystem)))